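; Player controller for the player ship, forwarding fire and orbit-movement input and handling the pause menu.
; On BeginPlay it caches the possessed BP_PlayerShip, then passes the Fire action and MoveAlongOrbit axis straight to it.
; TogglePause, triggered by the PauseGame action, creates or removes WBP_PauseMenu while switching game pause, input mode and mouse cursor.
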(event `self.ReceiveBeginPlay`
  (bind _asbp_player_ship (cast `/Game/Blueprints/GameObjects/BP_PlayerShip` (`self.K2_GetPawn`)))
  (set `self.PlayerShipRef` _asbp_player_ship))

(event `InputAction|PauseGame` :paused true
  (params (Key :type "Key Structure"))
  (:`Pressed`
    (`self.Toggle Pause`)))

(event `Toggle Pause`
  (if (`self.IsPaused`)
    (`Widget.RemoveFromParent` (`self.PauseMenuWidget `))
    (`GameplayStatics.SetGamePaused` false)
    (`WidgetBlueprintLibrary.SetInputMode_GameOnly` (`GameplayStatics.GetPlayerController` 0))
    (set `self.bShowMouseCursor` false)
    (set `self.IsPaused` false)
    (else
      (bind _returnvalue (`|CreateWidget` "/Game/Blueprints/WBP_PauseMenu.WBP_PauseMenu_C" (`GameplayStatics.GetPlayerController` 0)))
      (bind _output_get (set `self.PauseMenuWidget ` _returnvalue))
      (`UserWidget.AddToViewport` _output_get 0)
      (`GameplayStatics.SetGamePaused` true)
      (`WidgetBlueprintLibrary.SetInputMode_GameAndUIEx` (`GameplayStatics.GetPlayerController` 0) _returnvalue)
      (set `self.bShowMouseCursor` true)
      (set `self.IsPaused` true))))

(event `InputAction|Fire`
  (params (Key :type "Key Structure"))
  (:`Pressed`
    (`PlayerShip.Fire` (`self.PlayerShipRef`))))

(event `InputAxis|MoveAlongOrbit`
  (params (AxisValue :type "Float (single-precision)"))
  (`PlayerShip.MoveAlongOrbit` (`self.PlayerShipRef`) AxisValue))

(fn `UserConstructionScript`)