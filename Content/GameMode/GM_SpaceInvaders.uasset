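; Game mode Blueprint for Space Invaders that shows the end screens when the game is lost or won.
; The OnGameOverUI and OnGameWonUI events create WBP_GameOver and WBP_GameWon respectively and add them to the viewport.
; Both events also switch the first player controller to UI-only input and show the mouse cursor.
; It holds no other logic, and nothing in this graph calls either event.
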(event `self.OnGameOverUI`
  (bind _returnvalue (`GameplayStatics.GetPlayerController` 0))
  (`WidgetBlueprintLibrary.SetInputMode_UIOnlyEx` _returnvalue null)
  (set `PlayerController.bShowMouseCursor` true _returnvalue)
  (bind _returnvalue_2 (`|CreateWidget` "/Game/Blueprints/WBP_GameOver.WBP_GameOver_C"))
  (`UserWidget.AddToViewport` _returnvalue_2 0))

(event `self.OnGameWonUI`
  (bind _returnvalue (`GameplayStatics.GetPlayerController` 0))
  (bind _returnvalue_2 (`|CreateWidget` "/Game/Blueprints/WBP_GameWon.WBP_GameWon_C"))
  (`UserWidget.AddToViewport` _returnvalue_2 0)
  (`WidgetBlueprintLibrary.SetInputMode_UIOnlyEx` _returnvalue null)
  (set `PlayerController.bShowMouseCursor` true _returnvalue))

(fn `UserConstructionScript`)